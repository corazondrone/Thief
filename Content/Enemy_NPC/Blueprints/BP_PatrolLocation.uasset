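; BP_PatrolLocation is a placeable patrol point marker for enemy NPCs, tagged with a zone assignment.
; On BeginPlay it registers its collision sphere's world location and zone with the LilThiefGM game mode, which stores patrol locations in an array.
; The construction script shows the zone on a debug text component.
; A disconnected leftover of the same registration targets BP_ThirdPersonGameMode and never runs.
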(event `self.ReceiveBeginPlay`
  ;[1 1 1] Save Patrol Location to Array located in GameMode
  (bind _aslil_thief_gm (cast `/Game/LilThief/LilThiefGM` (`GameplayStatics.GetGameMode`)))
  (`/Game/LilThief/LilThiefGM.StorePatrolLocations` _aslil_thief_gm (`SceneComponent.K2_GetComponentLocation` (`self.Collision_Sphere`)) (`self.Zone Assignment`)))

(fn `UserConstructionScript`
  (`TextRenderComponent.K2_SetText` (`self.DebugText-Zone`) (`KismetTextLibrary.Conv_StringToText` (`KismetStringLibrary.Concat_StrStr` "Zone : " (`KismetStringLibrary.Conv_IntToString` (`self.Zone Assignment`))))))