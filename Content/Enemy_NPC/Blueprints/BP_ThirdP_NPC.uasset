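; Enemy NPC character for LilThief that patrols an assigned zone, then chases and shoots at the player on sight.
; Looping timers drive patrol between random GameMode zone points, pausing for each move and random wait.
; PawnSensing pauses patrol and starts pursuit with projectile fire, suppressed when gassed; a range timer resumes patrol after a delay once the player escapes.
; Modular body meshes follow the main mesh's pose.
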(event OnSeePawn(PawnSensing)
  (params (Pawn :type Pawn%20Object%20Reference))
  ;[1 0.1562 0.1562] If Player is detected, pause Patrol Timer
  (Variables|Patrol|SetPlayerDebugDetection true)
  (Utilities|FlowControl|Delay 0.3)
  (Variables|Patrol|SetPlayerDebugDetection false)
  (CallFunction|ResetPursuitTimer)
  (Utilities|Time|PauseTimerbyHandle (Variables|Patrol|GetTimerHandle_Patrol))
  ;[0.9792 0.0969 0.0969] Add +1 To Player Detection Counter
  (Utilities|FlowControl|Sequence
    (:then_0
      (Utilities|FlowControl|DoOnce false
        (:Completed
          (CallFunction|IncrementPlayerDetections 1))))
    (:then_1
      ;[1 0.1354 0.1354] Set Alert Timer. Detects if player is still within range.
      ; If player is within range, continue pursuit.
      ; If player exits range, cancel animations and restart Patrol Timer.
      (Utilities|FlowControl|DoOnce false
        (:Completed
          (bind _returnvalue (Utilities|Time|SetTimerbyEvent (delegate Custom|PursuitTimer) 0.1 true))
          (Variables|Patrol|SetTimerHandle_PlayerRange _returnvalue)
          (CallFunction|AlertSearch))))))

(event Custom|EnemyPatrol
  ;[1 0.09896 0.09896] Enemy Patrol Logic
  ;;[1 1 1] Pause Patrol Timer for later use.
  (Utilities|Time|PauseTimerbyHandle (Variables|Patrol|GetTimerHandle_Patrol))
  ;;[1 1 1] Choose Patrol Point from Saved Array.
  ;; Array is located in GameMode.
  (bind _patrollocation (CallFunction|ChoosePatrolPoint))
  (AI|AIMoveTo self _patrollocation 0 2e+01 false
    (:OnSuccess
      ;;[1 1 1] When Patrol Point is reached, use Patrol Timer value to wait before continuing patrol.
      ;; Patrol Timer is set in
      (Utilities|FlowControl|Delay (Variables|Patrol|GetPatrolTimer))
      (Utilities|Time|UnpauseTimerbyHandle (Variables|Patrol|GetTimerHandle_Patrol)))))

(event Custom|ResetDoOnceSpottedPlayer
  ;[0.4283 1 0.4172] Enemy Spots Player
  (Utilities|FlowControl|DoOnce false) ; enters at Reset
)

(event Custom|Patrol
  ;[1 0.1406 0.1406] Set Looping Patrol Timer
  (CallFunction|EnemyPatrol))

(event Custom|AlertSearch
  ;[1 0.2148 0.165] Enemy Pursue Attack Player
  (if (Variables|Default|GetKnockedOutByGas)
    (Variables|Default|SetIsFiring false)
    (else
      (Transformation|SetActorRotation self (Math|Rotator|MakeRotator 0.0 0.0 (.yaw (Math|Interpolation|RInterpTo (Transformation|GetActorRotation) (Math|Rotator|FindLookatRotation (Transformation|GetActorLocation) (Transformation|GetActorLocation)) (Utilities|Time|GetWorldDeltaSeconds) 0.3))))
      (Variables|Default|SetAimWeapon true)
      (AI|AIMoveTo self "0, 0, 0" (Game|GetPlayerCharacter 0) 2e+01 false
        (:then
          (CallFunction|FireonPlayer))))))

(event Custom|FireOnPlayer
  ;[1 0.07812 0.07812] Fire On Player
  (if (Variables|Default|GetKnockedOutByGas)
    (Variables|Default|SetIsFiring false)
    (elif (and (>= (Transformation|GetDistanceTo (Game|GetPlayerCharacter 0) self) 4e+01) (== (Variables|Patrol|GetisPlayerInRange?) false))
      (Game|SpawnActorfromClass "/Game/Enemy_NPC/Meshes/Enemy_NPC_Props/Projectile.Projectile_C" (Transformation|GetWorldTransform (Variables|Default|GetBulletSpawnLoc)) "Undefined" 0 self)
      (Audio|PlaySoundatLocation "/Game/Sound_Effects/WEAPONS/SciFi/Blasters_Simple/BLASTER_Deep_Muffled_stereo.BLASTER_Deep_Muffled_stereo" "0, 0, 0" "0, 0, 0" 1.0 1.0 0.0 0 0 0 0))))

(event Custom|Reset%20Pursuit%20Timer
  ;[1 0.1354 0.1354] Set Alert Timer. Detects if player is still within range.
  ; If player is within range, continue pursuit.
  ; If player exits range, cancel animations and restart Patrol Timer.
  (Utilities|FlowControl|DoOnce false) ; enters at Reset
)

(event Custom|PursuitTimer
  (bind _returnvalue (Game|GetPlayerCharacter 0))
  (bind _self self)
  (bind _returnvalue_2 (Transformation|GetDistanceTo _returnvalue _self))
  ;[1 0.1354 0.1354] Set Alert Timer. Detects if player is still within range.
  ; If player is within range, continue pursuit.
  ; If player exits range, cancel animations and restart Patrol Timer.
  (if (>= _returnvalue_2 3e+03)
    (Variables|Patrol|SetPursuit_DistanceToPlayer _returnvalue_2)
    (Variables|Patrol|SetisPlayerInRange? true)
    ;[1 0.1406 0.1406] If player exits range, cancel animations and cancel Pursuit Timer.
    (Class|NavMovementComponent|StopActiveMovement (Variables|Character|GetCharacterMovement))
    (Variables|Default|SetAimWeapon false)
    (Variables|Default|SetIsFiring false)
    (Utilities|Time|ClearandInvalidateTimerbyHandle (Variables|Patrol|GetTimerHandle_PlayerRange))
    (CallFunction|ResetPlayerDetectionCounter)
    ;[1 0.1406 0.1406] Wait before returning to Patrol Timer
    (Utilities|FlowControl|Delay (Variables|Patrol|GetResetPatrolTimer))
    (Utilities|Time|UnpauseTimerbyHandle (Variables|Patrol|GetTimerHandle_Patrol))
    (else
      (Variables|Patrol|SetisPlayerInRange? false))))

(event Custom|Reset%20Player%20Detection%20Counter
  ;[0.9792 0.0969 0.0969] Add +1 To Player Detection Counter
  (Utilities|FlowControl|DoOnce false) ; enters at Reset
)

(event EventTick
  (params (DeltaSeconds :type Float%20%28single-precision%29))
  ;[0.3843 0.298 1] Patrol Debug Info
)

(event EventBeginPlay
  ;[1 0.1302 0.1302] Saves a reference to GameMode
  (|SaveReferencetoLilThiefGameMode)
  (Components|SkinnedMesh|SetLeaderPoseComponent (Variables|Default|GetHands) (Variables|Character|GetMesh) false false)
  ;[1 0.1406 0.1406] Loops Through BP_PatrolPoint actors and saves each location into an array.
  ; Array is located in GameMode.
  (CallFunction|SavePatrolPoints)
  ;[1 0.1406 0.1406] Set Looping Patrol Timer
  (bind _returnvalue (Utilities|Time|SetTimerbyEvent (delegate Custom|Patrol) 0.1 true))
  (Variables|Patrol|SetTimerHandle_Patrol _returnvalue))

(fn ConstructionScript
  ;[1 1 1] Debug Text --
  ; Used for displaying numbers above Patrol Enemies
  ; Disconnect from Construction Script to prevent updates to text
  ; or
  ; Set visibility of TextRenderComponent to 'Hidden'
  (switch int (Variables|Patrol|Zone|GetZoneAssignment)
    (:1
      (Rendering|Components|TextRender|SetText (Variables|Default|GetDebugText-Zone) (Utilities|Text|ToText(String) (Utilities|String|Append "Zone : " (Utilities|String|ToString(Text) (Utilities|Text|MakeLiteralText "1"))))))
    (:2
      (Rendering|Components|TextRender|SetText (Variables|Default|GetDebugText-Zone) (Utilities|Text|ToText(String) (Utilities|String|Append "Zone : " (Utilities|String|ToString(Text) (Utilities|Text|MakeLiteralText "2"))))))
    (:3
      (Rendering|Components|TextRender|SetText (Variables|Default|GetDebugText-Zone) (Utilities|Text|ToText(String) (Utilities|String|Append "Zone : " (Utilities|String|ToString(Text) (Utilities|Text|MakeLiteralText "3"))))))
    (:4
      (Rendering|Components|TextRender|SetText (Variables|Default|GetDebugText-Zone) (Utilities|Text|ToText(String) (Utilities|String|Append "Zone : " (Utilities|String|ToString(Text) (Utilities|Text|MakeLiteralText "4"))))))
    (:5
      (Rendering|Components|TextRender|SetText (Variables|Default|GetDebugText-Zone) (Utilities|Text|ToText(String) (Utilities|String|Append "Zone : " (Utilities|String|ToString(Text) (Utilities|Text|MakeLiteralText "5"))))))
    (:6
      (Rendering|Components|TextRender|SetText (Variables|Default|GetDebugText-Zone) (Utilities|Text|ToText(String) (Utilities|String|Append "Zone : " (Utilities|String|ToString(Text) (Utilities|Text|MakeLiteralText "6"))))))
    (:7
      (Rendering|Components|TextRender|SetText (Variables|Default|GetDebugText-Zone) (Utilities|Text|ToText(String) (Utilities|String|Append "Zone : " (Utilities|String|ToString(Text) (Utilities|Text|MakeLiteralText "7"))))))))

(fn SavePatrolPoints
  (switch int (Variables|Patrol|Zone|GetZoneAssignment)
    (:1
      (bind _aslil_thief_gm (Utilities|Casting|CastToLilThiefGM (Game|GetGameMode)))
      (Variables|Patrol|Zone|SetZone1 (Variables|/Game/LilThief/LilThiefGM.LilThiefGM_C|GetZone1 _aslil_thief_gm))
      (Variables|Patrol|SetTotalPatrolPoints (Utilities|Array|Length (Variables|/Game/LilThief/LilThiefGM.LilThiefGM_C|GetZone1 _aslil_thief_gm)))
      (return))
    (:2
      (bind _aslil_thief_gm_2 (Utilities|Casting|CastToLilThiefGM (Game|GetGameMode)))
      (Variables|Patrol|Zone|SetZone2 (Variables|/Game/LilThief/LilThiefGM.LilThiefGM_C|GetZone2 _aslil_thief_gm_2))
      (Variables|Patrol|SetTotalPatrolPoints (Utilities|Array|Length (Variables|/Game/LilThief/LilThiefGM.LilThiefGM_C|GetZone2 _aslil_thief_gm_2)))
      (return))
    (:3
      (bind _aslil_thief_gm_3 (Utilities|Casting|CastToLilThiefGM (Game|GetGameMode)))
      (Variables|Patrol|Zone|SetZone3 (Variables|/Game/LilThief/LilThiefGM.LilThiefGM_C|GetZone3 _aslil_thief_gm_3))
      (Variables|Patrol|SetTotalPatrolPoints (Utilities|Array|Length (Variables|/Game/LilThief/LilThiefGM.LilThiefGM_C|GetZone3 _aslil_thief_gm_3)))
      (return))
    (:4
      (bind _aslil_thief_gm_4 (Utilities|Casting|CastToLilThiefGM (Game|GetGameMode)))
      (Variables|Patrol|Zone|SetZone4 (Variables|/Game/LilThief/LilThiefGM.LilThiefGM_C|GetZone4 _aslil_thief_gm_4))
      (Variables|Patrol|SetTotalPatrolPoints (Utilities|Array|Length (Variables|/Game/LilThief/LilThiefGM.LilThiefGM_C|GetZone4 _aslil_thief_gm_4)))
      (return))
    (:5
      (bind _aslil_thief_gm_5 (Utilities|Casting|CastToLilThiefGM (Game|GetGameMode)))
      (Variables|Patrol|Zone|SetZone5 (Variables|/Game/LilThief/LilThiefGM.LilThiefGM_C|GetZone5 _aslil_thief_gm_5))
      (Variables|Patrol|SetTotalPatrolPoints (Utilities|Array|Length (Variables|/Game/LilThief/LilThiefGM.LilThiefGM_C|GetZone5 _aslil_thief_gm_5)))
      (return))
    (:6
      (bind _aslil_thief_gm_6 (Utilities|Casting|CastToLilThiefGM (Game|GetGameMode)))
      (Variables|Patrol|Zone|SetZone6 (Variables|/Game/LilThief/LilThiefGM.LilThiefGM_C|GetZone6 _aslil_thief_gm_6))
      (Variables|Patrol|SetTotalPatrolPoints (Utilities|Array|Length (Variables|/Game/LilThief/LilThiefGM.LilThiefGM_C|GetZone6 _aslil_thief_gm_6)))
      (return))
    (:7
      (bind _aslil_thief_gm_7 (Utilities|Casting|CastToLilThiefGM (Game|GetGameMode)))
      (Variables|Patrol|Zone|SetZone7 (Variables|/Game/LilThief/LilThiefGM.LilThiefGM_C|GetZone7 _aslil_thief_gm_7))
      (Variables|Patrol|SetTotalPatrolPoints (Utilities|Array|Length (Variables|/Game/LilThief/LilThiefGM.LilThiefGM_C|GetZone7 _aslil_thief_gm_7)))
      (return))))

(fn ChoosePatrolPoint
  ;[1 1 1] Set Walk speed of Enemy Patrol
  (Variables|/Script/Engine.CharacterMovementComponent|SetMaxWalkSpeed (Variables|Character|GetCharacterMovement) 2e+02)
  ;[1 1 1] Set Random Patrol Time within range.
  ; This adds variety to each Patrol Time, keeping the player guessing.
  (Variables|Patrol|SetPatrolTimer (Math|Random|RandomFloatinRange 1.0 1e+01))
  (switch int (Variables|Patrol|Zone|GetZoneAssignment)
    (:1
      (return (Utilities|Array|Get(acopy) (Variables|Patrol|Zone|GetZone1) (Math|Random|RandomInteger (Math|Integer|Clamp(Integer) (Utilities|Array|Length (Variables|Patrol|Zone|GetZone1)) 1 3)))))
    (:2
      (return (Utilities|Array|Get(acopy) (Variables|Patrol|Zone|GetZone2) (Math|Random|RandomInteger (Math|Integer|Clamp(Integer) (Utilities|Array|Length (Variables|Patrol|Zone|GetZone2)) 1 3)))))
    (:3
      (return (Utilities|Array|Get(acopy) (Variables|Patrol|Zone|GetZone3) (Math|Random|RandomInteger (Math|Integer|Clamp(Integer) (Utilities|Array|Length (Variables|Patrol|Zone|GetZone3)) 1 3)))))
    (:4
      (return (Utilities|Array|Get(acopy) (Variables|Patrol|Zone|GetZone4) (Math|Random|RandomInteger (Math|Integer|Clamp(Integer) (Utilities|Array|Length (Variables|Patrol|Zone|GetZone4)) 1 3)))))
    (:5
      (return (Utilities|Array|Get(acopy) (Variables|Patrol|Zone|GetZone5) (Math|Random|RandomInteger (Math|Integer|Clamp(Integer) (Utilities|Array|Length (Variables|Patrol|Zone|GetZone5)) 1 3)))))
    (:6
      (return (Utilities|Array|Get(acopy) (Variables|Patrol|Zone|GetZone6) (Math|Random|RandomInteger (Math|Integer|Clamp(Integer) (Utilities|Array|Length (Variables|Patrol|Zone|GetZone6)) 1 3)))))
    (:7
      (return (Utilities|Array|Get(acopy) (Variables|Patrol|Zone|GetZone7) (Math|Random|RandomInteger (Math|Integer|Clamp(Integer) (Utilities|Array|Length (Variables|Patrol|Zone|GetZone7)) 1 3)))))))

(fn DebugPatrolPoints
  (params (Choose%20Debug%20Info :type Integer))
  (switch int Choose%20Debug%20Info
    (:1
      ;[0.4765 0.4022 1] Debug -- Print Patrol Locations
      (for _array_element (Variables|Patrol|Zone|GetZone1)
        (Development|PrintString (Utilities|String|ToString(Vector) _array_element))))
    (:2
      ;[0.4765 0.4022 1] Debug -- Print Distance to Player if Detected
      (if (Variables|Patrol|GetisPlayerInRange?)
        (Development|PrintString (Utilities|String|Append "Distance To Player = " (Utilities|String|ToString(Float) (Variables|Patrol|GetPursuit_DistanceToPlayer))))))
    (:3
      ;[0.4765 0.4022 1] Debug -- Print Number of Player Detections
      (if (Variables|Patrol|GetPlayerDebugDetection)
        (Utilities|FlowControl|DoOnce false
          (:Completed
            (Development|PrintString (Utilities|String|Append "Player Has Been Detected" "(" (Utilities|String|ToString(Integer) (Variables|Default|GetNumberofDetections)) ")" " Times"))))))
    (:4
      ;[0.3141 0.2581 0.901] Comment
      (if (Variables|Patrol|GetPlayerDebugDetection)
        (Utilities|FlowControl|DoOnce false
          (:Completed
            (Rendering|Components|TextRender|SetText (Variables|Default|GetDebugText-Zone) (Variables|Patrol|Zone|GetText_DebugZoneSelection))))))))

(fn IncrementPlayerDetections
  (params (Increment :type Integer))
  (Variables|Default|SetNumberofDetections (+ (Variables|Default|GetNumberofDetections) Increment)))