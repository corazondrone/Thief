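; Master enemy NPC character that patrols, spots the thief player through PawnSensing, then chases and shoots.
; Modular body, clothing and hair meshes follow the main mesh's pose.
; Patrol loops between one of two target-point pairs; a once-gated sighting increments the player's spotted count and starts pursuit.
; Firing repeats projectile spawns until the player is 1500 units away, then patrol resumes after a delay; gas knockout blocks firing.
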(event `self.ReceiveBeginPlay`
  (`SkinnedMeshComponent.SetLeaderPoseComponent` (`self.Hands`) (`self.Mesh`) false false)
  (`SkinnedMeshComponent.SetLeaderPoseComponent` (`self.Feet`) (`self.Mesh`) false false)
  (`SkinnedMeshComponent.SetLeaderPoseComponent` (`self.Lower`) (`self.Mesh`) false false)
  (`SkinnedMeshComponent.SetLeaderPoseComponent` (`self.Upper`) (`self.Mesh`) false false)
  (`SkinnedMeshComponent.SetLeaderPoseComponent` (`self.Upper Addon2`) (`self.Mesh`) false false)
  (`SkinnedMeshComponent.SetLeaderPoseComponent` (`self.Upper Addon3`) (`self.Mesh`) false false)
  (`SkinnedMeshComponent.SetLeaderPoseComponent` (`self.Upper Addon`) (`self.Mesh`) false false)
  (`SkinnedMeshComponent.SetLeaderPoseComponent` (`self.Lower Addon`) (`self.Mesh`) false false)
  (`SkinnedMeshComponent.SetLeaderPoseComponent` (`self.Hat1`) (`self.Mesh`) false false)
  (`SkinnedMeshComponent.SetLeaderPoseComponent` (`self.Hat2`) (`self.Mesh`) false false)
  (`SkinnedMeshComponent.SetLeaderPoseComponent` (`self.Hair`) (`self.Mesh`) false false)
  (`self.EnemyPatrol`))

(event `EnemyPatrol`
  ;[1 1 1] Enemy_Patrol
  (set `CharacterMovementComponent.MaxWalkSpeed` 200.0 (`self.CharacterMovement`))
  (if (`self.PatrolPathMain`)
    (`|AIMoveTo` self (0.0 0.0 0.0) (`self.TargetPoint_1`)
      (:`OnSuccess`
        (`KismetSystemLibrary.RetriggerableDelay` 2.0)
        (`|AIMoveTo` self (0.0 0.0 0.0) (`self.TargetPoint_2`)
          (:`OnSuccess`
            (`KismetSystemLibrary.RetriggerableDelay` 2.0)
            (`self.EnemyPatrol`)))))
    (else
      (`|AIMoveTo` self (0.0 0.0 0.0) (`self.TargetPoint_3`)
        (:`OnSuccess`
          (`KismetSystemLibrary.RetriggerableDelay` 2.0)
          (`|AIMoveTo` self (0.0 0.0 0.0) (`self.TargetPoint_4`)
            (:`OnSuccess`
              (`KismetSystemLibrary.RetriggerableDelay` 2.0)
              (`self.EnemyPatrol`))))))))

(event `self.PawnSensing.OnSeePawn`
  (params (Pawn :type "Pawn Object Reference"))
  ;[1 1 1] Enemy Spots Player
  (bind _aslil_thief_bp (cast `/Game/LilThief/LilThiefBP` Pawn))
  (`/Engine/EditorBlueprintResources/StandardMacros.DoOnce` false :!label _label
    (:`Completed`
      (set `/Game/LilThief/LilThiefBP.PlayerSpotted` (+ (`/Game/LilThief/LilThiefBP.PlayerSpotted` _aslil_thief_bp) 1) _aslil_thief_bp)
      (set `self.PlayerDetected` true)
      (`self.AlertSearch`))))

(event `ResetDoOnceSpottedPlayer`
  ;[1 1 1] Enemy Spots Player
  (goto _label :!via `Reset`))

(event `AlertSearch`
  (bind (_returnvalue_roll _returnvalue_pitch _returnvalue_yaw) (`KismetMathLibrary.BreakRotator` (`KismetMathLibrary.RInterpTo` (`self.K2_GetActorRotation`) (`KismetMathLibrary.FindLookAtRotation` (`self.K2_GetActorLocation`) (`self.K2_GetActorLocation`)) (`GameplayStatics.GetWorldDeltaSeconds`) 0.3)))
  ;[1 1 1] Enemy Pursue Attack Player
  (if (`self.KnockedOutByGas`)
    (set `self.IsFiring` false)
    (else
      (`self.K2_SetActorRotation` self (`KismetMathLibrary.MakeRotator` 0.0 0.0 _returnvalue_yaw) false)
      (set `self.AimWeapon` true)
      (`|AIMoveTo` self (0.0 0.0 0.0) (`GameplayStatics.GetPlayerCharacter` 0) 20.0
        (:`then`
          (if (`self.PlayerDetected`)
            (`self.FireOnPlayer`)))))))

(event `FireOnPlayer`
  (if (`self.KnockedOutByGas`)
    (set `self.IsFiring` false)
    (elif (>= (`self.GetDistanceTo` (`GameplayStatics.GetPlayerCharacter` 0) self) 1500.0)
      (set `self.PlayerDetected` false)
      (`KismetSystemLibrary.RetriggerableDelay` 15.0)
      (set `self.AimWeapon` false)
      (`self.ResetDoOnceSpottedPlayer`)
      (`self.EnemyPatrol`)
      (else
        (`|SpawnActorFromClass` "/Game/Enemy_NPC/Meshes/Enemy_NPC_Props/Projectile.Projectile_C" (`SceneComponent.K2_GetComponentToWorld` (`self.BulletSpawnLoc`)) "Undefined" "OverrideRootScale" null self)
        (`GameplayStatics.PlaySound2D` "/Game/Sound_Effects/WEAPONS/SciFi/Plasma_Cannons/PLASMA_CANNON_Zap_Dropping_Tail_mono.PLASMA_CANNON_Zap_Dropping_Tail_mono" 1.0 1.0 0.0 null null)
        (`KismetSystemLibrary.Delay` 0.8)
        (set `self.IsFiring` true)
        (`KismetSystemLibrary.Delay` 0.1)
        (set `self.IsFiring` false)
        (if (`self.PlayerDetected`)
          (`self.FireOnPlayer`))))))

(fn `UserConstructionScript`)